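; Light-based stealth Blueprint that decides whether MyCharacter is hidden from the level's point lights.
; Every Tick it loops over all PointLight actors and, for those within a fixed range, line-traces on Visibility to the player's lowered location.
; A blocked trace counts as hidden, and the first clear trace breaks the loop.
; The result, which persists when no light is in range, sets the character's IsHidden and prints a debug message when hidden.
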(event Custom|BreakLoop
  ;[1 1 1] Loop through all Point Lights/location of
  (Utilities|Array|ForEachLoopwithBreak (stale EventTick _outactors)) ; enters at Break
)

(event EventTick
  (params (DeltaSeconds :type Float%20%28single-precision%29))
  ;[1 1 1] Get MyCharacter/location of
  (bind _asmy_character (Utilities|Casting|CastToMyCharacter (Game|GetPlayerCharacter 0)))
  (Variables|Default|SetMyCharacterRef _asmy_character)
  (Variables|Default|SetplayerLocation (- (Transformation|GetActorLocation _asmy_character) "0, 0,88.000000"))
  ;[1 1 1] Loop through all Point Lights/location of
  (bind _outactors (Actor|GetAllActorsOfClass "/Script/Engine.PointLight"))
  (bind _array_element (Utilities|Array|ForEachLoopwithBreak _outactors)
    (:LoopBody
      (Variables|Default|SetlightLocation (Transformation|GetActorLocation _array_element))
      ;[1 1 1] If light is inRange[true]
      (bind _output_get (Variables|Default|SetinRange (< (Math|Vector|VectorLength (- (Variables|Default|GetplayerLocation) (Variables|Default|GetlightLocation))) 1.5e+03)))
      (if _output_get
        ;[1 1 1] Trace from light to player
        (bind _outhit (Collision|LineTraceByChannel (Variables|Default|GetlightLocation) (Variables|Default|GetplayerLocation) "TraceTypeQuery1" false 0 "None"))
        ;[1 1 1] If collides with player = playerHidden[false/breakloop]
        (if (.bBlockingHit (Collision|BreakHitResult _outhit))
          (bind _output_get_2 (Variables|Default|SetplayerHidden true))
          (else
            (Variables|Default|SetplayerHidden false)))
        (if (not _output_get_2)
          (CallFunction|BreakLoop))))
    (:Completed
      ;[1 1 1] If playerHidden[true] = isHidden[true]
      (if (Variables|Default|GetplayerHidden)
        (Variables|/Game/MVP/MyCharacter.MyCharacter_C|SetisHidden (Variables|Default|GetMyCharacterRef) true)
        (Development|PrintString "HIDDEN")
        (else
          (Variables|/Game/MVP/MyCharacter.MyCharacter_C|SetisHidden (Variables|Default|GetMyCharacterRef) false))))))

(fn ConstructionScript)